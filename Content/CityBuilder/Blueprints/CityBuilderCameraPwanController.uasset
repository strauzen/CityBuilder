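; City-builder controller that drives the CameraPawn with keyboard/axis movement, screen-edge scrolling, rotation and zoom.
; On BeginPlay it caches the player pawn; movement helpers offset it along its local axes at a constant root height, with speed scaled by spring-arm length and a fast-move multiplier.
; Holding Pan opens gates for yaw and clamped pitch while blocking movement and edge scrolling.
; Zoom steps the clamped arm length, with resets for zoom and rotation.
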(event `self.ReceiveBeginPlay`
  (`|ExecutionSequence`
    (:`then_0`
      (`self.ReferenceCasts`))))

(event `InputAxis|MoveForward`
  (params (AxisValue :type "Float (single-precision)"))
  ;[1 1 1] Movement X
  (if (not (`self.DisableCamNav`))
    (`self.K2_SetActorTransform` (`self.CameraPwanRef`) (`self.ConstantHeight` (`self.MovementX` AxisValue (`self.MovementSpeedCalculation`) (`self.FastMoveMultiplier`) (`self.CameraPwanRef`)) (`self.CameraRootHeight`)) false false)))

(event `InputAxis|MoveRight`
  (params (AxisValue :type "Float (single-precision)"))
  ;[1 1 1] Movement Y
  (if (not (`self.DisableCamNav`))
    (`self.K2_SetActorTransform` (`self.CameraPwanRef`) (`self.ConstantHeight` (`self.MovementY` AxisValue (`self.MovementSpeedCalculation`) (`self.FastMoveMultiplier`) (`self.CameraPwanRef`)) (`self.CameraRootHeight`)) false false)))

(event `InputAction|PanReset`
  (params (Key :type "Key Structure" :default "AnyKey"))
  (bind _camerapwanref (`self.CameraPwanRef`))
  ;[1 1 1] Pan reset
  (:`Pressed`
    (`self.K2_SetActorRotation` _camerapwanref (`KismetMathLibrary.MakeRotator` (.roll (`self.K2_GetActorRotation` _camerapwanref))) false)))

(event `InputAxis|Yaw`
  (params (AxisValue :type "Float (single-precision)"))
  ;[1 1 1] Pan X
  (`/Engine/EditorBlueprintResources/StandardMacros.Gate` true :!label _label
    (:`Exit`
      (`self.K2_SetActorRotation` (`self.CameraPwanRef`) (`KismetMathLibrary.MakeRotator` (.roll (`self.K2_GetActorRotation` (`self.CameraPwanRef`))) (.pitch (`self.K2_GetActorRotation` (`self.CameraPwanRef`))) (+ (.yaw (`self.K2_GetActorRotation` (`self.CameraPwanRef`))) (* (`self.PanSensitivity`) AxisValue))) false))))

(event `InputAction|Pan`
  (params (Key :type "Key Structure" :default "AnyKey"))
  ;[1 1 1] Pan X
  (:`Pressed`
    (set `self.DisableCamNav` true)
    (goto _label :!via `Open`))
  (:`Released`
    (set `self.DisableCamNav` false)
    (goto _label :!via `Close`)))

(event `InputAction|FastMove`
  (params (Key :type "Key Structure" :default "AnyKey"))
  ;[1 1 1] Move multiplier
  (:`Pressed`
    (set `self.FastMoveMultiplier` 2.0))
  (:`Released`
    (set `self.FastMoveMultiplier` 1.0)))

(event `InputAxis|Pitch`
  (params (AxisValue :type "Float (single-precision)"))
  ;[1 1 1] Pan Y
  (`/Engine/EditorBlueprintResources/StandardMacros.Gate` true :!label _label_2
    (:`Exit`
      (`self.K2_SetActorRotation` (`self.CameraPwanRef`) (`KismetMathLibrary.MakeRotator` (.roll (`self.K2_GetActorRotation` (`self.CameraPwanRef`))) (`KismetMathLibrary.FClamp` (+ (.pitch (`self.K2_GetActorRotation` (`self.CameraPwanRef`))) (* (`self.PanSensitivity`) AxisValue)) (`self.PitchHigherAngle`) (`self.PitchLowerAngle`)) (.yaw (`self.K2_GetActorRotation` (`self.CameraPwanRef`)))) false))))

(event `InputAction|Pan`
  (params (Key :type "Key Structure" :default "AnyKey"))
  ;[1 1 1] Pan Y
  (:`Pressed`
    (set `self.DisableCamNav` true)
    (goto _label_2 :!via `Open`))
  (:`Released`
    (set `self.DisableCamNav` false)
    (goto _label_2 :!via `Close`)))

(event `InputAction|ZoomIn`
  (params (Key :type "Key Structure" :default "AnyKey"))
  (bind _springarm (`/Game/CityBuilder/Blueprints/CameraPawn.SpringArm` (`self.CameraPwanRef`)))
  ;[1 1 1] Zoom in/out
  (:`Pressed`
    (set `SpringArmComponent.TargetArmLength` (`KismetMathLibrary.FClamp` (- (`SpringArmComponent.TargetArmLength` _springarm) (`self.ZoomSensitivity`)) 500.0 (`self.MaxArmDistance`)) _springarm)))

(event `InputAxisKey|MouseX`
  (params (AxisValue :type "Float (single-precision)"))
  ;[1 1 1] Edge movement
  (if (not (`self.DisableCamNav`))
    (bind (_deltaxspeed _deltayspeed) (`self.ScreenEdgeMovement` :!label _label_3))
    (`self.K2_AddActorLocalOffset` (`self.CameraPwanRef`) (`KismetMathLibrary.MakeVector` _deltaxspeed _deltayspeed) true false)))

(event `InputAxisKey|MouseY`
  (params (AxisValue :type "Float (single-precision)"))
  ;[1 1 1] Edge movement
  (if (not (`self.DisableCamNav`))
    (goto _label_3 :!via `MouseY`)))

(event `InputAction|ZoomOut`
  (params (Key :type "Key Structure" :default "AnyKey"))
  (bind _springarm (`/Game/CityBuilder/Blueprints/CameraPawn.SpringArm` (`self.CameraPwanRef`)))
  ;[1 1 1] Zoom in/out
  (:`Pressed`
    (set `SpringArmComponent.TargetArmLength` (`KismetMathLibrary.FClamp` (+ (`self.ZoomSensitivity`) (`SpringArmComponent.TargetArmLength` _springarm)) 500.0 (`self.MaxArmDistance`)) _springarm)))

(event `InputAction|ZoomReset`
  (params (Key :type "Key Structure" :default "AnyKey"))
  ;[1 1 1] Reset zoom
  (:`Pressed`
    (set `SpringArmComponent.TargetArmLength` 1500.0 (`/Game/CityBuilder/Blueprints/CameraPawn.SpringArm` (`self.CameraPwanRef`)))))

(fn `MovementSpeedCalculation`
  (returns (MoveSensitivity :type "Float (double-precision)"))
  (return (`KismetMathLibrary.FClamp` (/ (`SpringArmComponent.TargetArmLength` (`/Game/CityBuilder/Blueprints/CameraPawn.SpringArm` (`self.CameraPwanRef`))) 100.0) 5.0 20.0)))

(fn `UserConstructionScript`)
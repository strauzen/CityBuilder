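; BP_GhostBuilding is a ghost building for the city builder that displays the mesh of a given building.
; OnSpawn, ignored while the ghost is active, stores the display mesh, building class and construction proxy, then applies the mesh to SMGhostBuilding.
; KillGhost clears those references and the active flag without destroying the actor or resetting the component's mesh, so OnSpawn can set it up again.
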(event `OnSpawn`
  (params (DisplayMesh :type "StaticMesh Object Reference") (BuildingClass :type "/Game/CityBuilder/Blueprints/Buildings/BP_BuildingMaster Class Reference") (ConstructionProxy :type "/Game/CityBuilder/Blueprints/Construction/BP_ConstructionProxy Class Reference"))
  (if (not (`self.IsActive`))
    (set `self.DisplayMesh` DisplayMesh)
    (set `self.BuildingClass` BuildingClass)
    (set `self.ConstructionProxy` ConstructionProxy)
    (set `self.IsActive` true)
    (`StaticMeshComponent.SetStaticMesh` (`self.SM_GhostBuilding`) (`self.DisplayMesh`))))

(event `KillGhost`
  (set `self.DisplayMesh` null)
  (set `self.BuildingClass` null)
  (set `self.ConstructionProxy` null)
  (set `self.IsActive` false))

(fn `UserConstructionScript`)